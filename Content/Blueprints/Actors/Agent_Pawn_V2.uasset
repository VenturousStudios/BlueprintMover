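; Player pawn prototype on the Mover plugin that acts as its own input producer and implements walking movement math in Blueprint.
; Enhanced Input drives look and fills WalkInputs, which ProduceInput packs into the Mover input collection.
; WalkGenerateMoveMutable traces the floor, tilts camera-relative direction onto it, and proposes linear and angular velocity using a hand-written ComputeVelocity.
; A child-actor functional test, shared with Walking_MovementMode_V2, asserts intermediate results; FindFloor is an empty stub.
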(event Input|EnhancedActionEvents|EnhancedInputActionMouseXY_IA
  (params (ActionValue :type Vector%202D%20Structure) (ElapsedSeconds :type Float%20%28double-precision%29) (TriggeredSeconds :type Float%20%28double-precision%29) (InputAction :type Input%20Action%20Object%20Reference :default "/Game/Blueprints/Input/MouseXY_IA.MouseXY_IA"))
  (Pawn|Input|AddControllerYawInput (.x ActionValue))
  (Pawn|Input|AddControllerPitchInput (.y ActionValue)))

(event Input|EnhancedActionEvents|EnhancedInputActionMoveXY_IA
  (params (ActionValue :type Vector%202D%20Structure) (ElapsedSeconds :type Float%20%28double-precision%29) (TriggeredSeconds :type Float%20%28double-precision%29) (InputAction :type Input%20Action%20Object%20Reference :default "/Game/Blueprints/Input/MoveXY_IA.MoveXY_IA"))
  (bind _camera (Variables|Default|GetCamera))
  (bind _returnvalue (Transformation|GetWorldRotation _camera))
  (:Triggered
    (bind _structout (Utilities|Struct|SetmembersinCharacterDefaultInputs (Variables|Default|GetWalkInputs) "DirectionalIntent" (Math|Vector|MakeVector (.x ActionValue) (.y ActionValue) 0.0) _returnvalue))
    (Class|FunctionalTest|AssertEqualVector2D (Variables|Default|GetMoverTest) (Math|Vector2D|MakeVector2D (.x (.MoveInput (Utilities|Struct|BreakCharacterDefaultInputs _structout))) (.y (.MoveInput (Utilities|Struct|BreakCharacterDefaultInputs _structout)))) (Math|Vector2D|MakeVector2D 0.0 0.0) "Expected to be clamped between -1 and 1" 1.0))
  (:Canceled
    (Utilities|Struct|SetmembersinCharacterDefaultInputs (Variables|Default|GetWalkInputs) "DirectionalIntent" (Math|Vector|MakeVector 0.0 0.0 0.0) _returnvalue :!label _label))
  (:Completed
    (goto _label)))

(event EventBeginPlay
  (Input|AddMappingContext (PlayerController|LocalPlayerSubsystems|GetEnhancedInputLocalPlayerSubsystem (Game|GetPlayerController 0)) "/Game/Blueprints/Input/BaseMovement_IMC.BaseMovement_IMC" 0 "(bIgnoreAllPressedKeysUntilRelease=True,bForceImmediately=False,bNotifyUserSettings=False)")
  (Variables|/Script/Mover.MoverComponent|SetInputProducer (Variables|Default|GetCharacterMover) self)
  ;[1 1 1] UpdateMoverTest
  (bind _asmover_functional_test (Utilities|Casting|CastToMover_FunctionalTest (Variables|/Script/Engine.ChildActorComponent|GetChildActor (Variables|Default|GetFunctionalTest))))
  (Variables|/Game/Blueprints/Mover/Walking_MovementMode_V2.Walking_MovementMode_V2_C|SetMoverTest (Class|MoverComponent|FindMovementMode (Variables|Default|GetCharacterMover) "/Game/Blueprints/Mover/Walking_MovementMode_V2.Walking_MovementMode_V2_C") _asmover_functional_test)
  (Variables|Default|SetMoverTest _asmover_functional_test))

(fn ConstructionScript)

(fn ComputeVelocity
  (params (DeltaSeconds :type Float%20%28double-precision%29) (PriorVelocity :type Vector) (MoveDirection :type Vector) (MaxSpeed :type Float%20%28double-precision%29) (TurningBoost :type Float%20%28double-precision%29) (Deceleration :type Float%20%28double-precision%29) (Acceleration :type Float%20%28double-precision%29) (Friction :type Float%20%28double-precision%29))
  (bind _returnvalue (Math|Vector|VectorClampSizeMax MoveDirection 1.0))
  (LocalVariables|SetAnalogInputModifier (select (> (Math|Vector|VectorLengthSquared _returnvalue) 0.0) (Math|Vector|VectorLength _returnvalue) 0.0))
  (LocalVariables|SetMaxPawnSpeed (* MaxSpeed (LocalVariables|GetAnalogInputModifier)))
  (LocalVariables|SetExceedingMaxSpeed (> (Math|Vector|VectorLengthSquared PriorVelocity) (* (Math|Float|Square MaxSpeed) 1.01)))
  (if (Math|Boolean|ANDBoolean (> (LocalVariables|GetAnalogInputModifier) 0.0) (not (LocalVariables|GetExceedingMaxSpeed)) (> (Math|Vector|VectorLengthSquared PriorVelocity) 0.0))
    (return (+ PriorVelocity (* (- (* (Math|Vector|VectorClampSizeMax MoveDirection 1.0) (Math|Vector|VectorLength PriorVelocity)) PriorVelocity) (Math|Float|Min(Float) (* (Math|Float|Clamp(Float) (* DeltaSeconds TurningBoost)) Friction) 1.0))))
    (else
      (Utilities|FlowControl|Sequence
        (:then_0
          (if (> (Math|Vector|VectorLengthSquared PriorVelocity) 0.0)
            (LocalVariables|SetTempVelocity (* (Math|Vector|Normalize PriorVelocity) (Math|Float|Max(Float) (- (Math|Vector|VectorLength PriorVelocity) (* (Math|Float|Absolute(Float) (+ (* (Math|Vector|VectorLength PriorVelocity) Friction) Deceleration)) DeltaSeconds)) 0.0))))
          (if (and (LocalVariables|GetExceedingMaxSpeed) (> (Math|Vector|VectorLengthSquared (LocalVariables|GetTempVelocity)) (Math|Float|Square (LocalVariables|GetMaxPawnSpeed))))
            (LocalVariables|SetTempVelocity (* (Math|Vector|Normalize PriorVelocity) (LocalVariables|GetMaxPawnSpeed)))))
        (:then_1
          (LocalVariables|SetExceedingMaxSpeed (> (Math|Vector|VectorLengthSquared (LocalVariables|GetTempVelocity)) (* (Math|Float|Square MaxSpeed) 1.01)))
          (return (Math|Vector|VectorClampSizeMax (* (Math|Vector|VectorClampSizeMax MoveDirection 1.0) (Math|Float|Absolute(Float) Acceleration) DeltaSeconds) (select (LocalVariables|GetExceedingMaxSpeed) (Math|Vector|VectorLength (LocalVariables|GetTempVelocity)) (LocalVariables|GetMaxPawnSpeed)))))))))

(fn WalkMoveDirection
  (bind _walkinputs (Variables|Default|GetWalkInputs))
  (bind _camera (Variables|Default|GetCamera))
  (bind _moveinput (Utilities|Struct|BreakCharacterDefaultInputs _walkinputs))
  (return (Class|KismetMathLibrary|VectorNormal2D (+ (* (Math|Vector|GetRightVector _camera) (.x _moveinput)) (* (Math|Vector|GetForwardVector _camera) (.y _moveinput))) 0.0001)))

(fn FindFloor
  (params (FloorSweepDistance :type Float%20%28double-precision%29) (UpdatedPrimitive :type Primitive%20Component%20Object%20Reference) (Location :type Vector :default "0, 0, 0") (MaxWalkSlopeCosine :type Float%20%28double-precision%29))
  (return ""))

(fn ProduceInput
  (params (SimTimeMs :type Integer))
  (bind _structout (Utilities|Struct|SetmembersinCharacterDefaultInputs (Variables|Default|GetWalkInputs) "DirectionalIntent"))
  (Class|MoverDataCollectionLibrary|AddDatatoCollection (Variables|Default|GetWalkInputCollection) _structout)
  (return (Utilities|Struct|MakeMoverInputCmdContext (Variables|Default|GetWalkInputCollection))))

(fn WalkGenerateMoveMutable
  (params (StartState :type Mover%20Tick%20Start%20Data%20Structure%20%28by%20ref%29) (TimeStep :type Mover%20Time%20Step%20Structure%20%28by%20ref%29))
  (Utilities|FlowControl|Sequence
    (:then_0
      (bind (_outhit _returnvalue) (Collision|LineTraceByChannel (+ (Transformation|GetActorLocation) (LocalVariables|GetMoveDirection)) (+ (+ (Transformation|GetActorLocation) (LocalVariables|GetMoveDirection)) "0.000000,0.000000,-96.000000") "TraceTypeQuery1" false 0 "None")) ; We need to Trace to get data about the floor.
      (LocalVariables|SetMovementNormal (select _returnvalue (.ImpactNormal (Collision|BreakHitResult _outhit)) "0.000000,0.000000,1.000000"))
      (LocalVariables|SetMoveDirection (CallFunction|WalkMoveDirection)) ; Used in multiple places. Better to cache.
      (bind (_didsucceed _targetasrawbytes) (Class|MoverDataCollectionLibrary|GetDatafromCollection (.SyncStateCollection (Utilities|Struct|BreakMoverSyncState (.syncstate StartState)))))
      (Class|FunctionalTest|AssertTrue (Variables|Default|GetMoverTest) _didsucceed "StartingSyncState - Get 
Data From Collection Failed")
      (LocalVariables|SetStartingSyncState _targetasrawbytes)
      (LocalVariables|SetCommonSettings (Class|MoverComponent|FindSharedSettingsBP (Variables|Default|GetCharacterMover) "/Script/Mover.CommonLegacyMovementSettings"))
      (LocalVariables|SetPriorVelocity (Math|Vector|ProjectVectorontoPlane (.Velocity (Utilities|Struct|BreakMoverDefaultSyncState (LocalVariables|GetStartingSyncState))) (LocalVariables|GetMovementNormal)))
      (if (and (> (Math|Vector|VectorLengthSquared (LocalVariables|GetMoveDirection)) 0.0) (not (> (Math|Vector|VectorLengthSquared (LocalVariables|GetPriorVelocity)) (* (Math|Float|Square (Variables|/Script/Mover.CommonLegacyMovementSettings|GetMaxSpeed (LocalVariables|GetCommonSettings))) 1.01))))
        (LocalVariables|SetFriction (Variables|/Script/Mover.CommonLegacyMovementSettings|GetGroundFriction (LocalVariables|GetCommonSettings)))
        (else
          (LocalVariables|SetFriction (* (select (Variables|/Script/Mover.CommonLegacyMovementSettings|GetbUseSeparateBrakingFriction (LocalVariables|GetCommonSettings)) (Variables|/Script/Mover.CommonLegacyMovementSettings|GetBrakingFriction (LocalVariables|GetCommonSettings)) (Variables|/Script/Mover.CommonLegacyMovementSettings|GetGroundFriction (LocalVariables|GetCommonSettings))) (Variables|/Script/Mover.CommonLegacyMovementSettings|GetBrakingFrictionFactor (LocalVariables|GetCommonSettings)))))))
    (:then_1
      (bind _returnvalue_2 (Class|MovementUtils|ConstraintoPlane (LocalVariables|GetMoveDirection) (Class|KismetMathLibrary|MakePlanefromPointandNormal "0, 0, 0" (LocalVariables|GetMovementNormal)) true)) ; Tilt the MoveDirection vector if the floor is not flat.
      (LocalVariables|SetMoveDirection _returnvalue_2) ; CAUTION: Maybe not needed
      (Utilities|String|LogString "Debug Move Intent" (CallFunction|TraceDirectionDebug (Transformation|GetActorLocation) _returnvalue_2 100 0.2))
      (bind _velocity (CallFunction|ComputeVelocity (* (.stepms TimeStep) 0.001) (LocalVariables|GetPriorVelocity) (LocalVariables|GetMoveDirection) (Variables|/Script/Mover.CommonLegacyMovementSettings|GetMaxSpeed (LocalVariables|GetCommonSettings)) (Variables|/Script/Mover.CommonLegacyMovementSettings|GetTurningBoost (LocalVariables|GetCommonSettings)) (Variables|/Script/Mover.CommonLegacyMovementSettings|GetDeceleration (LocalVariables|GetCommonSettings)) (Variables|/Script/Mover.CommonLegacyMovementSettings|GetAcceleration (LocalVariables|GetCommonSettings)) (LocalVariables|GetFriction))) ; Computes actual velocity. Maybe\nuse branch before to check if the\nVelocity will be 0?
      (LocalVariables|SetMovePlaneVelocity _velocity)
      (Class|FunctionalTest|AssertNotEqualVector (Variables|Default|GetMoverTest) _velocity "0, 0, 0" "Should be different than 0,0,0 if there is input.") ; Used to check if we are providing input. Should be reworked after we\nmake walking mode work.
      (bind _returnvalue_3 (Class|MovementUtils|ConstraintoPlane (LocalVariables|GetMovePlaneVelocity) (Class|KismetMathLibrary|MakePlanefromPointandNormal "0, 0, 0" (LocalVariables|GetMovementNormal)) true)) ; Tilt the MovePlaneVelocity vector if the floor is not flat.\nTEST if it is necessary.
      (LocalVariables|SetLinearVelocity _returnvalue_3)
      (bind _returnvalue_4 (Class|MovementUtils|ComputeAngularVelocity (.Orientation (Utilities|Struct|BreakMoverDefaultSyncState (LocalVariables|GetStartingSyncState))) (Math|Conversions|RotationFromXVector (LocalVariables|GetMoveDirection)) (* (.stepms TimeStep) 0.001) (Variables|/Script/Mover.CommonLegacyMovementSettings|GetTurningRate (LocalVariables|GetCommonSettings)))) ; Needed to compute angular velocity if the orientation\nis different. Maybe have a branch before to check if\nthe orientation is different?
      (Class|FunctionalTest|AssertNotEqualRotator (Variables|Default|GetMoverTest) _returnvalue_4 "0, 0, 0" "Should be something other than 0 if 
orientation is changing.")
      (return (Utilities|Struct|MakeProposedMove "AdditiveVelocity" "None" (not (Math|Vector|VectorIsNearlyZero (LocalVariables|GetMoveDirection))) false (LocalVariables|GetMoveDirection) (LocalVariables|GetLinearVelocity) _returnvalue_4 (LocalVariables|GetMovePlaneVelocity))))))