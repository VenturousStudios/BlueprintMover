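; Player pawn on the Mover plugin, with Enhanced Input mouse look and apparently work-in-progress walking movement.
; The move action stores a fixed +Y directional intent, ignoring its value, and ProduceInput passes it to CharacterMover.
; WalkGenerateMoveMutable builds ground-move parameters from input, sync state, traced normal and shared settings for ComputeControlledGroundMove.
; FindFloor hand-builds a capsule-sweep floor check; an older trace-and-slide movement graph is left disconnected.
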(event Input|EnhancedActionEvents|EnhancedInputActionMouseXY_IA
  (params (ActionValue :type Vector%202D%20Structure) (ElapsedSeconds :type Float%20%28double-precision%29) (TriggeredSeconds :type Float%20%28double-precision%29) (InputAction :type Input%20Action%20Object%20Reference :default "/Game/Blueprints/Input/MouseXY_IA.MouseXY_IA"))
  (Pawn|Input|AddControllerYawInput (.x ActionValue))
  (Pawn|Input|AddControllerPitchInput (.y ActionValue)))

(event Input|EnhancedActionEvents|EnhancedInputActionMoveXY_IA
  (params (ActionValue :type Vector%202D%20Structure) (ElapsedSeconds :type Float%20%28double-precision%29) (TriggeredSeconds :type Float%20%28double-precision%29) (InputAction :type Input%20Action%20Object%20Reference :default "/Game/Blueprints/Input/MoveXY_IA.MoveXY_IA"))
  (|SetBy-RefVar (Variables|Default|GetCharInputs) (Utilities|Struct|MakeCharacterDefaultInputs "DirectionalIntent" "0.000000,1.000000,0.000000" "1.000000,0.000000,0.000000")))

(event EventBeginPlay
  (Input|AddMappingContext (PlayerController|LocalPlayerSubsystems|GetEnhancedInputLocalPlayerSubsystem (Game|GetPlayerController 0)) "/Game/Blueprints/Input/BaseMovement_IMC.BaseMovement_IMC" 0 "(bIgnoreAllPressedKeysUntilRelease=True,bForceImmediately=False,bNotifyUserSettings=False)")
  (Variables|/Script/Mover.MoverComponent|SetInputProducer (Variables|Default|GetCharacterMover) self)
  (Class|MoverDataCollectionLibrary|AddDatatoCollection (Variables|Default|GetMoverDataCollection) (Variables|Default|GetCharInputs)))

(fn ConstructionScript)

(fn FindFloor
  (params (FloorSweepDistance :type Float%20%28double-precision%29) (UpdatedPrimitive :type Primitive%20Component%20Object%20Reference) (Location :type Vector :default "0, 0, 0") (MaxWalkSlopeCosine :type Float%20%28double-precision%29))
  (bind _ascapsule_collision (Utilities|Casting|CastToCapsuleComponent UpdatedPrimitive)
    (:then
      (LocalVariables|SetCapsuleHalfHeight (Variables|/Script/Engine.CapsuleComponent|GetCapsuleHalfHeight _ascapsule_collision))
      (LocalVariables|SetCapsuleRadius (Variables|/Script/Engine.CapsuleComponent|GetCapsuleRadius _ascapsule_collision))
      (LocalVariables|SetShrinkHeight (* (- (Variables|/Script/Engine.CapsuleComponent|GetCapsuleHalfHeight _ascapsule_collision) (Variables|/Script/Engine.CapsuleComponent|GetCapsuleRadius _ascapsule_collision)) 0.1))
      (LocalVariables|SetTraceDist (+ FloorSweepDistance (LocalVariables|GetShrinkHeight)))
      (LocalVariables|SetSweepDirection (Math|Vector|MakeVector 0.0 0.0 (* -1.0 (LocalVariables|GetTraceDist))))
      (Utilities|FlowControl|Sequence
        (:then_0
          (bind (_outhit _returnvalue) (Collision|CapsuleTraceByChannel Location (+ Location (LocalVariables|GetSweepDirection)) (LocalVariables|GetCapsuleRadius) (- (LocalVariables|GetCapsuleHalfHeight) (LocalVariables|GetShrinkHeight)) "TraceTypeQuery1" false 0 "None"))
          (LocalVariables|SetHit _outhit)
          (LocalVariables|SetbBlockingHit _returnvalue))
        (:then_1
          (if (LocalVariables|GetbBlockingHit)
            (if (or (.bInitialOverlap (Collision|BreakHitResult (LocalVariables|GetHit))) (not (< (Class|KismetMathLibrary|VSizeXYSquared (- (.ImpactPoint (Collision|BreakHitResult (LocalVariables|GetHit))) Location)) (Math|Float|Max(Float) 0.15 (- (LocalVariables|GetCapsuleRadius) 0.15)))))
              (LocalVariables|SetCapsuleRadius (Math|Float|Max(Float) 0.0 (- (LocalVariables|GetCapsuleRadius) 0.15)))
              (if (not (or (Math|Float|NearlyEqual(Float) (LocalVariables|GetCapsuleHalfHeight) 0.0 0.01) (Math|Float|NearlyEqual(Float) (LocalVariables|GetCapsuleRadius) 0.0 0.01)))
                (LocalVariables|SetShrinkHeight (* (- (LocalVariables|GetCapsuleHalfHeight) (LocalVariables|GetCapsuleRadius)) 0.9))
                (LocalVariables|SetTraceDist (+ FloorSweepDistance (LocalVariables|GetShrinkHeight)))
                (LocalVariables|SetSweepDirection (Math|Vector|MakeVector 0.0 0.0 (* -1.0 (LocalVariables|GetTraceDist))))
                (LocalVariables|SetCapsuleHalfHeight (Math|Float|Max(Float) (- (LocalVariables|GetCapsuleHalfHeight) (LocalVariables|GetShrinkHeight)) (LocalVariables|GetCapsuleRadius)))
                (LocalVariables|SetHit "")
                ;[1 1 1] Duplicate
                (bind (_outhit_2 _returnvalue_2) (Collision|CapsuleTraceByChannel Location (+ Location (LocalVariables|GetSweepDirection)) (LocalVariables|GetCapsuleRadius) (- (LocalVariables|GetCapsuleHalfHeight) (LocalVariables|GetShrinkHeight)) "TraceTypeQuery1" false 0 "None"))
                (LocalVariables|SetHit _outhit_2)
                (LocalVariables|SetbBlockingHit _returnvalue_2)))
            (else
              (LocalVariables|SetMaxPenetrationAdjust (Math|Float|Max(Float) 2.4 (LocalVariables|GetCapsuleRadius)))
              (LocalVariables|SetSweepResult (Math|Float|Max(Float) (- 0.0 (LocalVariables|GetMaxPenetrationAdjust)) (- (* (.Time (Collision|BreakHitResult (LocalVariables|GetHit))) (LocalVariables|GetTraceDist)) (LocalVariables|GetShrinkHeight))))
              (LocalVariables|SetFloorResult (Utilities|Struct|MakeFloorCheckResult_Editable_Struct (and (.bblockinghit (LocalVariables|GetHit)) (not (.binitialoverlap (LocalVariables|GetHit)))) false false 0.0 (LocalVariables|GetSweepResult) (LocalVariables|GetHit)))
              (bind _returnvalue_3 (Class|FloorQueryUtils|IsHitSurfaceWalkable (LocalVariables|GetHit) MaxWalkSlopeCosine))
              (if (and _returnvalue_3 (and (.bBlockingHit (Collision|BreakHitResult (LocalVariables|GetHit))) (not (.bInitialOverlap (Collision|BreakHitResult (LocalVariables|GetHit))))))
                (if (<= (LocalVariables|GetSweepResult) FloorSweepDistance)
                  (bind _structout (Utilities|Struct|SetmembersinFloorCheckResult_Editable_Struct (LocalVariables|GetFloorResult) true))
                  (return _structout))))))))
    (:CastFailed
      (Development|PrintString "FIND FLOOR FAIL! 
PRIMITIVE IS NOT CAPSULE" true true "(R=1.000000,G=0.000000,B=0.000000,A=1.000000)" 15.0))))

(fn ProduceInput
  (params (SimTimeMs :type Integer))
  (Class|MoverDataCollectionLibrary|AddDatatoCollection (.inputcollection (Class|MoverComponent|GetLastInputCmd (Variables|Default|GetCharacterMover))) (Variables|Default|GetCharInputs))
  (return (Class|MoverComponent|GetLastInputCmd (Variables|Default|GetCharacterMover))))

(fn WalkGenerateMoveMutable
  (params (StartState :type Mover%20Tick%20Start%20Data%20Structure%20%28by%20ref%29) (TimeStep :type Mover%20Time%20Step%20Structure%20%28by%20ref%29))
  (bind (_inputcmd _syncstate) (Utilities|Struct|BreakMoverTickStartData StartState))
  (bind _returnvalue (Transformation|GetActorLocation))
  (bind _charactermover (Variables|Default|GetCharacterMover))
  (bind _charactermover_2 (Variables|Default|GetCharacterMover))
  (bind _groundparams_editable (Variables|Default|GetGroundParams_Editable))
  (bind _returnvalue_2 (Class|MoverComponent|FindSharedSettingsBP _charactermover_2 "/Script/Mover.CommonLegacyMovementSettings"))
  (bind _returnvalue_3 (Class|MoverComponent|FindSharedSettingsBP _charactermover "/Script/Mover.CommonLegacyMovementSettings"))
  (bind _brakingfrictionfactor (Variables|/Script/Mover.CommonLegacyMovementSettings|GetBrakingFrictionFactor _returnvalue_3))
  (bind (_didsucceed _targetasrawbytes) (Class|MoverDataCollectionLibrary|GetDatafromCollection (.inputcollection _inputcmd)))
  (if _didsucceed
    (Variables|Default|SetCharacterInputs _targetasrawbytes)
    (bind (_didsucceed_2 _targetasrawbytes_2) (Class|MoverDataCollectionLibrary|GetDatafromCollection (.syncstatecollection _syncstate)))
    (if _didsucceed_2
      (Variables|Default|SetStartSyncState _targetasrawbytes_2)
      (Utilities|FlowControl|Sequence
        (:then_0
          (Variables|Default|SetDeltaSeconds (* (.StepMs (Utilities|Struct|BreakMoverTimeStep TimeStep)) 0.001))
          (Variables|Default|SetBlackboard_Mutable (Class|MoverComponent|GetSimBlackboard (Variables|Default|GetCharacterMover)))
          (bind (_outhit _returnvalue_4) (Collision|LineTraceByChannel _returnvalue (+ _returnvalue "0.000000,0.000000,-96.000000") "TraceTypeQuery1" false 0 "None"))
          (if _returnvalue_4
            (Variables|Default|SetMovementNormal (.ImpactNormal (Collision|BreakHitResult _outhit)))
            (else
              (bind _returnvalue_5 (Class|MoverComponent|GetUpDirection (Variables|Default|GetCharacterMover)))
              (Variables|Default|SetMovementNormal _returnvalue_5))))
        (:then_1
          (if (Math|Vector|VectorIsNearlyZero (.OrientationIntent (Utilities|Struct|BreakCharacterDefaultInputs (Variables|Default|GetCharacterInputs))))
            (Variables|Default|SetIntendedOrientation_WorldSpace (.Orientation (Utilities|Struct|BreakMoverDefaultSyncState (Variables|Default|GetStartSyncState))))
            (else
              (Variables|Default|SetIntendedOrientation_WorldSpace (Math|Conversions|RotationFromXVector (.MoveInput (Utilities|Struct|BreakCharacterDefaultInputs (Variables|Default|GetCharacterInputs))))))))
        (:then_2
          (Utilities|Struct|SetmembersinGroundParams_Struct _groundparams_editable (.MoveInputType (Utilities|Struct|BreakCharacterDefaultInputs (Variables|Default|GetCharacterInputs))))
          (Utilities|Struct|SetmembersinGroundParams_Struct _groundparams_editable (.MoveInput (Utilities|Struct|BreakCharacterDefaultInputs (Variables|Default|GetCharacterInputs)))))
        (:then_3
          (Utilities|Struct|SetmembersinGroundParams_Struct (Variables|Default|GetGroundParams_Editable) (Variables|Default|GetIntendedOrientation_WorldSpace) (Math|Vector|ProjectVectorontoPlane (.Velocity (Utilities|Struct|BreakMoverDefaultSyncState (Variables|Default|GetStartSyncState))) (Variables|Default|GetMovementNormal)) (.Orientation (Utilities|Struct|BreakMoverDefaultSyncState (Variables|Default|GetStartSyncState))) (Variables|/Script/Mover.CommonLegacyMovementSettings|GetMaxSpeed _returnvalue_2) (Variables|/Script/Mover.CommonLegacyMovementSettings|GetAcceleration _returnvalue_2) (Variables|/Script/Mover.CommonLegacyMovementSettings|GetDeceleration _returnvalue_2) (Variables|/Script/Mover.CommonLegacyMovementSettings|GetTurningRate _returnvalue_2) (Variables|/Script/Mover.CommonLegacyMovementSettings|GetTurningBoost _returnvalue_2) (Variables|Default|GetMovementNormal) (Variables|Default|GetDeltaSeconds)))
        (:then_4
          (bind _returnvalue_6 (Class|MovementUtils|IsExceedingMaxSpeed (.PriorVelocity (Utilities|Struct|BreakGroundParams_Struct (Variables|Default|GetGroundParams_Editable))) (Variables|/Script/Mover.CommonLegacyMovementSettings|GetMaxSpeed (Class|MoverComponent|FindSharedSettingsBP (Variables|Default|GetCharacterMover) "/Script/Mover.CommonLegacyMovementSettings"))))
          (if (and (not _returnvalue_6) (> (Math|Vector|VectorLengthSquared (.MoveInput (Utilities|Struct|BreakGroundParams_Struct (Variables|Default|GetGroundParams_Editable)))) 0.0))
            (Utilities|Struct|SetmembersinGroundParams_Struct (Variables|Default|GetGroundParams_Editable) (Variables|/Script/Mover.CommonLegacyMovementSettings|GetGroundFriction (Class|MoverComponent|FindSharedSettingsBP (Variables|Default|GetCharacterMover) "/Script/Mover.CommonLegacyMovementSettings")))
            (elif (Variables|/Script/Mover.CommonLegacyMovementSettings|GetbUseSeparateBrakingFriction _returnvalue_3)
              (Utilities|Struct|SetmembersinGroundParams_Struct (Variables|Default|GetGroundParams_Editable) (* (Variables|/Script/Mover.CommonLegacyMovementSettings|GetBrakingFriction _returnvalue_3) _brakingfrictionfactor))
              (else
                (Utilities|Struct|SetmembersinGroundParams_Struct (Variables|Default|GetGroundParams_Editable) (* _brakingfrictionfactor (Variables|/Script/Mover.CommonLegacyMovementSettings|GetGroundFriction _returnvalue_3)))))))
        (:then_5
          (bind _returnvalue_7 (Class|StructUtilsFunctionLibrary|MakeInstancedStruct (Variables|Default|GetParams)))
          (Class|StructUtilsFunctionLibrary|SetInstancedStructValue _returnvalue_7 (Variables|Default|GetGroundParams_Editable))
          (bind _value (Class|StructUtilsFunctionLibrary|GetInstancedStructValue _returnvalue_7)
            (:Valid
              (bind _returnvalue_8 (Class|GroundMovementUtils|ComputeControlledGroundMove _value))
              (return _returnvalue_8)))))
      (else
        (Development|PrintString "28 - StartSyncState GET DATA FAILED" true true "(R=1.000000,G=0.000000,B=0.000000,A=1.000000)" 15.0)))
    (else
      (Development|PrintString "28 - CharacterInputs GET DATA FAILED" true true "(R=1.000000,G=0.000000,B=0.000000,A=1.000000)" 15.0))))