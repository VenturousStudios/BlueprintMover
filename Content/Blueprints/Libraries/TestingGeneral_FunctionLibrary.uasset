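; Blueprint function library of debug helpers for visualising traces and string arrays during testing.
; TraceDirectionDebug draws a timed Camera-channel line trace from a start point along a scaled direction, always returning true regardless of the hit.
; PrintArrayDebug prints each string for a given duration, coloured by index through a ten-step rainbow from red to magenta.
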(fn TraceDirectionDebug
  (params (StartLocation :type Vector%20%28by%20ref%29) (Direction :type Vector%20%28by%20ref%29) (Length :type Integer) (Time :type Float%20%28double-precision%29))
  (Collision|LineTraceByChannel 0 StartLocation (+ StartLocation (* Direction Length)) "TraceTypeQuery2" false 0 "ForDuration" true "(R=0.039216,G=0.000000,B=1.000000,A=1.000000)" "(R=0.039216,G=0.000000,B=1.000000,A=1.000000)" Time)
  (return true))

(fn PrintArrayDebug
  (params (StringArray :type Array%20of%20Strings) (PrintDuration :type Float%20%28double-precision%29))
  (for _index (range 0 (- (Utilities|Array|Length StringArray) 1))
    (Development|PrintString 0 (Utilities|Array|Get(acopy) StringArray _index) true true (Utilities|Select :Index _index :Option%200 "(R=1.000000,G=0.000000,B=0.000000,A=1.000000)" :Option%201 "(R=1.000000,G=0.550000,B=0.000000,A=1.000000)" :Option%202 "(R=0.900000,G=1.000000,B=0.000000,A=1.000000)" :Option%203 "(R=0.350000,G=1.000000,B=0.000000,A=1.000000)" :Option%204 "(R=0.000000,G=1.000000,B=0.200000,A=1.000000)" :Option%205 "(R=0.000000,G=1.000000,B=0.750000,A=1.000000)" :Option%206 "(R=0.000000,G=0.700000,B=1.000000,A=1.000000)" :Option%207 "(R=0.000000,G=0.150000,B=1.000000,A=1.000000)" :Option%208 "(R=0.400000,G=0.000000,B=1.000000,A=1.000000)" :Option%209 "(R=0.950000,G=0.000000,B=1.000000,A=1.000000)") PrintDuration)))